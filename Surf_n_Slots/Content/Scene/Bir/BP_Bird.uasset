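; BP_Bird is a bird scene actor that moves through the level while playing a flipbook-style animation.
; BeginPlay runs an endless delayed loop that swaps the material on component E through three materials in a ping-pong order to animate it.
; Tick passes a frame-rate-scaled speed to MoveObjectInScene to move the actor each frame.
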(event EventBeginPlay
  (Rendering|Material|SetMaterial (Variables|Default|Gete) 0 (Variables|Default|GetNewVar) :!label _label)
  (Utilities|FlowControl|Delay 0.2)
  (Rendering|Material|SetMaterial (Variables|Default|Gete) 0 (Variables|Default|GetNewVar_0))
  (Utilities|FlowControl|Delay 0.2)
  (Rendering|Material|SetMaterial (Variables|Default|Gete) 0 (Variables|Default|GetNewVar_1))
  (Utilities|FlowControl|Delay 0.2)
  (Rendering|Material|SetMaterial (Variables|Default|Gete) 0 (Variables|Default|GetNewVar_0))
  (Utilities|FlowControl|Delay 0.2)
  (Rendering|Material|SetMaterial (Variables|Default|Gete) 0 (Variables|Default|GetNewVar))
  (goto _label))

(event Collision|EventActorBeginOverlap
  (params (OtherActor :type Actor%20Object%20Reference)))

(event EventTick
  (params (DeltaSeconds :type Float%20%28single-precision%29))
  (CallFunction|MoveObjectinScene (* DeltaSeconds 2e+02) self))

(fn ConstructionScript)