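; BP_Char is an actor that continuously cycles the material on its static mesh, producing a flipbook-style swap.
; From BeginPlay, a self-looping Delay chain steps a counter through a fixed range, wrapping it back to zero and advancing at a short fixed interval.
; NewFunction uses that counter to index the NewVar material array and applies the result to the mesh's first material slot.
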(event EventBeginPlay
  (if (>= (Variables|Default|GetNewVar_0) 14) :!label _label
    (Variables|Default|SetNewVar_0 0))
  (CallFunction|NewFunction (Variables|Default|GetNewVar_0))
  (Math|Integer|IncrementInt (Variables|Default|GetNewVar_0)
    (:%20%20
      (Utilities|FlowControl|Delay 0.2)
      (goto _label))))

(event Collision|EventActorBeginOverlap
  (params (OtherActor :type Actor%20Object%20Reference)))

(event EventTick
  (params (DeltaSeconds :type Float%20%28single-precision%29)))

(fn ConstructionScript)

(fn NewFunction
  (params (Dimension%201 :type Integer))
  (Rendering|Material|SetMaterial (Variables|Debug|GetStaticMeshComponent) 0 (Utilities|Array|Get(acopy) (Variables|Default|GetNewVar) Dimension%201)))