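; BP_Gamble is a clickable slot machine that rolls ingredients for building a dish.
; Clicking Cylinder_006 spends a round, resets picks, shows three random ingredients on WBP_Slot widgets and plays a rotation timeline.
; Three animated buttons call NewFunction to toggle their slot's ingredient in the dish array, spawning or destroying its actor.
; SpawnMoney spawns coins through a delayed loop, and Tick debug-prints the current dish.
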(event OnClicked(Cylinder_006)
  (params (TouchedComponent :type Primitive%20Component%20Object%20Reference) (ButtonPressed :type Key%20Structure :default "None"))
  ;[0.15 0.15 0.15 0.5] Spin Slots
  (CallFunction|SpinSlots))

(event OnClicked(Button_1)
  (params (TouchedComponent :type Primitive%20Component%20Object%20Reference) (ButtonPressed :type Key%20Structure :default "None"))
  ;[0.15 0.15 0.15 0.5] Buttons to add ingridient
  (Utilities|FlowControl|Sequence
    (:then_0
      (CallFunction|NewFunction))
    (:then_1
      (bind _newtrack_0 (Timeline|Timeline_0 PlayFromStart)
        (:Update
          (Transformation|SetRelativeLocation (Variables|Default|GetButton_1) (Math|Vector|MakeVector 0.0 (Math|Float|Lerp 0.0 -7.0 _newtrack_0) 0.0) false false))))))

(event OnClicked(Button_2)
  (params (TouchedComponent :type Primitive%20Component%20Object%20Reference) (ButtonPressed :type Key%20Structure :default "None"))
  ;[0.15 0.15 0.15 0.5] Buttons to add ingridient
  (Utilities|FlowControl|Sequence
    (:then_0
      (CallFunction|NewFunction 1))
    (:then_1
      (bind _newtrack_0 (Timeline|Timeline_1 PlayFromStart)
        (:Update
          (Transformation|SetRelativeLocation (Variables|Default|GetButton_2) (Math|Vector|MakeVector 0.0 (Math|Float|Lerp 0.0 -7.0 _newtrack_0) 0.0) false false))))))

(event OnClicked(Button_3)
  (params (TouchedComponent :type Primitive%20Component%20Object%20Reference) (ButtonPressed :type Key%20Structure :default "None"))
  ;[0.15 0.15 0.15 0.5] Buttons to add ingridient
  (Utilities|FlowControl|Sequence
    (:then_0
      (CallFunction|NewFunction 2))
    (:then_1
      (bind _newtrack_0 (Timeline|Timeline_2 PlayFromStart)
        (:Update
          (Transformation|SetRelativeLocation (Variables|Default|GetButton_3) (Math|Vector|MakeVector 0.0 (Math|Float|Lerp 0.0 -7.0 _newtrack_0) 0.0) false false))))))

(event Custom|SpinSlots
  (bind _ingridientadded_ (Variables|Default|GetIngridientAdded?))
  ;[0.15 0.15 0.15 0.5] Spin Slots
  (Variables|Default|SetDishGived? false)
  (if (> (Variables|Default|GetCurrentRoundsAmount) 0)
    (Math|Integer|DecrementInt (Variables|Default|GetCurrentRoundsAmount)
      (:%20%20
        (Utilities|FlowControl|Sequence
          (:then_0
            (for (_ _array_index) _ingridientadded_
              (Utilities|Array|SetArrayElem _ingridientadded_ _array_index false)))
          (:then_1
            (Utilities|Array|Clear (Variables|Default|GetCurrentSlotsArray))
            (bind _output (CallFunction|ChooseRandomIngridient (Variables|Default|GetWidget_1)))
            (Utilities|Array|Add (Variables|Default|GetCurrentSlotsArray) _output)
            (bind _output_2 (CallFunction|ChooseRandomIngridient (Variables|Default|GetWidget_2)))
            (Utilities|Array|Add (Variables|Default|GetCurrentSlotsArray) _output_2)
            (bind _output_3 (CallFunction|ChooseRandomIngridient (Variables|Default|GetWidget_3)))
            (Utilities|Array|Add (Variables|Default|GetCurrentSlotsArray) _output_3))
          (:then_2
            (bind _newtrack_0 (Timeline|Timeline PlayFromStart)
              (:Update
                (Transformation|SetRelativeRotation (Variables|Default|GetCylinder_006) (Math|Rotator|MakeRotator (Math|Float|Lerp 0.0 7e+01 _newtrack_0) 0.0 0.0) false false)))))))))

(event Custom|Spawn%20Money
  (params (LastIndex :type Integer))
  (Game|SpawnActorfromClass "/Game/Scene/BP_coin.BP_coin_C" (Math|Transform|MakeTransform (Transformation|GetWorldLocation (Variables|/Game/Scene/BP_CoinSpawner.BP_CoinSpawner_C|GetDefaultSceneRoot (Variables|Default|GetNewVar)))) "Undefined" "MultiplyWithRoot" 0 0 :!label _label)
  (Math|Integer|IncrementInt (Variables|Default|GetLast%20Index)
    (:%20%20
      (Utilities|FlowControl|Delay 0.05)
      (if (< (Variables|Default|GetLast%20Index) LastIndex)
        (goto _label)
        (else
          (Variables|Default|SetLast%20Index 0))))))

(event EventBeginPlay
  ;[0.15 0.15 0.15 0.5] BeginPlay
  (bind _asgs_core (Utilities|Casting|CastToGS_Core (Game|GetGameState)))
  (Variables|Default|SetAs%20GS%20Core _asgs_core))

(event EventTick
  (params (DeltaSeconds :type Float%20%28single-precision%29))
  (for _array_element (Variables|Default|GetCurrentDishArray)
    (Development|PrintString (Utilities|String|EnumtoString (.Name (Utilities|Struct|BreakS_IngridientsStruct (Utilities|GetClassDefaults _array_element)))) true true "(R=0.000000,G=0.660000,B=1.000000,A=1.000000)" DeltaSeconds)))

(fn ConstructionScript)

(fn ChooseRandomIngridient
  (params (self2 :type Widget%20Component%20Object%20Reference))
  (bind _ingridientsarray (Variables|Default|GetIngridientsArray))
  (LocalVariables|SetCurrentsSlotIngridieant (Utilities|Array|Get(acopy) _ingridientsarray (Math|Random|RandomIntegerinRange 0 (- (Utilities|Array|Length _ingridientsarray) 1))))
  (Default|SetImage (.AsWBP%20Slot (Utilities|Casting|CastToWBP_Slot (UserInterface|GetWidget self2))) (.Icon (Utilities|Struct|BreakS_IngridientsStruct (Utilities|GetClassDefaults (LocalVariables|GetCurrentsSlotIngridieant)))))
  (return (LocalVariables|GetCurrentsSlotIngridieant)))

(fn NewFunction
  (params (ArrayIndex_Slots :type Integer))
  (bind _currentslotsarray (Variables|Default|GetCurrentSlotsArray))
  (bind _currentslotsarray_2 (Variables|Default|GetCurrentSlotsArray))
  (bind _currentdisharray (Variables|Default|GetCurrentDishArray))
  (bind _currentdisharray_actors (Variables|Default|GetCurrentDishArray_Actors))
  (bind _output (Utilities|Array|Get(acopy) _currentslotsarray ArrayIndex_Slots))
  (bind _output_2 (Utilities|Array|Get(acopy) _currentslotsarray_2 ArrayIndex_Slots))
  (if (not (Variables|Default|GetDishGived?))
    (if (<= (Utilities|Array|Length (Variables|Default|GetCurrentDishArray)) 4)
      (if (Utilities|Array|Get(acopy) (Variables|Default|GetIngridientAdded?) ArrayIndex_Slots)
        (Utilities|Array|RemoveIndex _currentdisharray (Utilities|Array|FindItem _currentdisharray _output))
        (Utilities|Array|SetArrayElem (Variables|Default|GetIngridientAdded?) ArrayIndex_Slots false)
        (bind _returnvalue (Actor|GetActorOfClass _output))
        (Actor|DestroyActor (Utilities|Array|Get(acopy) _currentdisharray_actors (Utilities|Array|FindItem _currentdisharray_actors _returnvalue)))
        (else
          (Utilities|Array|Add (Variables|Default|GetCurrentDishArray) _output_2)
          (Utilities|Array|SetArrayElem (Variables|Default|GetIngridientAdded?) ArrayIndex_Slots true)
          (bind _returnvalue_2 (Game|SpawnActorfromClass (.Class_reference (Utilities|Struct|BreakS_IngridientsStruct (Utilities|GetClassDefaults _output_2))) (Math|Transform|MakeTransform (Utilities|Select :Index ArrayIndex_Slots :Option%200 (Transformation|GetWorldLocation (Variables|Default|GetArrow)) :Option%201 (Transformation|GetWorldLocation (Variables|Default|GetArrow1)) :Option%202 (Transformation|GetWorldLocation (Variables|Default|GetArrow2))) "0, 0, 0" "0.200000,0.200000,0.200000") "AlwaysSpawn" "MultiplyWithRoot" 0 "NewEnumerator0" 0))
          (Utilities|Array|Add (Variables|Default|GetCurrentDishArray_Actors) _returnvalue_2)
          (Development|PrintString (Utilities|String|ToString(Vector) (Transformation|GetWorldLocation (Variables|/Game/Ingridients/BP_Paren_Ingridient.BP_Paren_Ingridient_C|GetDefaultSceneRoot _returnvalue_2)))))))))