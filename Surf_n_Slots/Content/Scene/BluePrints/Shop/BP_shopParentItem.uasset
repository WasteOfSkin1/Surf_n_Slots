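; Base shop item actor that the player buys by clicking its static mesh.
; NewFunction casts self to the Tiki or Ingridient child class to read its price, then deducts it from GS_Core's CurrentMoney if affordable.
; On success, a Tiki adds its class to BP_Gamble's TikisArray and destroys itself.
; A Saouce item spawns its class at BP_Gamble's SaoceLocation and stays in place.
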(event OnClicked(StaticMesh)
  (params (TouchedComponent :type Primitive%20Component%20Object%20Reference) (ButtonPressed :type Key%20Structure :default "None"))
  (if (CallFunction|NewFunction)
    (switch Utilities|FlowControl|Switch|SwitchonE_ShopType (Variables|Default|GetShop_ItemType)
      (:NewEnumerator0
        (bind _asbp_parent_tiki (Utilities|Casting|CastToBP_Parent_Tiki self))
        (bind _returnvalue (Actor|GetActorOfClass "/Game/Scene/BluePrints/Objects/BP_Gamble.BP_Gamble_C"))
        (Utilities|Array|Add (Variables|/Game/Scene/BluePrints/Objects/BP_Gamble.BP_Gamble_C|GetTiki'sArray _returnvalue) (.Class_reference (Utilities|Struct|BreakS_TikiStruct (Variables|/Game/Tiki_Totems/BP_Parent_Tiki.BP_Parent_Tiki_C|GetData _asbp_parent_tiki))))
        (Actor|DestroyActor))
      (:NewEnumerator1
        (bind _returnvalue_2 (Actor|GetActorOfClass "/Game/Scene/BluePrints/Objects/BP_Gamble.BP_Gamble_C"))
        (bind _asbp_paren_ingridient (Utilities|Casting|CastToBP_Paren_Ingridient self))
        (Game|SpawnActorfromClass (.Class_reference (Utilities|Struct|BreakS_IngridientsStruct (Variables|/Game/Ingridients/BP_Paren_Ingridient.BP_Paren_Ingridient_C|GetIngridient_Data _asbp_paren_ingridient))) (Math|Transform|MakeTransform (Transformation|GetWorldLocation (Variables|/Game/Scene/BluePrints/Objects/BP_Gamble.BP_Gamble_C|GetSaoceLocation _returnvalue_2))) "Undefined" "MultiplyWithRoot" 0 0)))))

(event EventBeginPlay)

(event Collision|EventActorBeginOverlap
  (params (OtherActor :type Actor%20Object%20Reference)))

(event EventTick
  (params (DeltaSeconds :type Float%20%28single-precision%29)))

(fn ConstructionScript)

(fn NewFunction
  (bind _returnvalue (Game|GetGameState))
  (bind _returnvalue_2 (Game|GetGameState))
  (bind _self self)
  (bind _asgs_core (Utilities|Casting|CastToGS_Core _returnvalue))
  (bind _asgs_core_2 (Utilities|Casting|CastToGS_Core _returnvalue_2))
  (bind _asbp_parent_tiki (Utilities|Casting|CastToBP_Parent_Tiki _self)
    (:then
      (if (>= (Variables|/Game/Core/GS_Core.GS_Core_C|GetCurrentMoney _asgs_core_2) (.Price (Utilities|Struct|BreakS_TikiStruct (Variables|/Game/Tiki_Totems/BP_Parent_Tiki.BP_Parent_Tiki_C|GetData _asbp_parent_tiki))))
        (Variables|/Game/Core/GS_Core.GS_Core_C|SetCurrentMoney _asgs_core_2 (- (Variables|/Game/Core/GS_Core.GS_Core_C|GetCurrentMoney _asgs_core_2) (.Price (Utilities|Struct|BreakS_TikiStruct (Variables|/Game/Tiki_Totems/BP_Parent_Tiki.BP_Parent_Tiki_C|GetData _asbp_parent_tiki)))))
        (return true)
        (else
          (return false))))
    (:CastFailed
      (bind _asbp_paren_ingridient (Utilities|Casting|CastToBP_Paren_Ingridient _self))
      (if (>= (Variables|/Game/Core/GS_Core.GS_Core_C|GetCurrentMoney _asgs_core) (.Price (Utilities|Struct|BreakS_IngridientsStruct (Variables|/Game/Ingridients/BP_Paren_Ingridient.BP_Paren_Ingridient_C|GetIngridient_Data _asbp_paren_ingridient))))
        (Variables|/Game/Core/GS_Core.GS_Core_C|SetCurrentMoney _asgs_core (- (Variables|/Game/Core/GS_Core.GS_Core_C|GetCurrentMoney _asgs_core) (.Price (Utilities|Struct|BreakS_IngridientsStruct (Variables|/Game/Ingridients/BP_Paren_Ingridient.BP_Paren_Ingridient_C|GetIngridient_Data _asbp_paren_ingridient)))))
        (return true)
        (else
          (return false))))))