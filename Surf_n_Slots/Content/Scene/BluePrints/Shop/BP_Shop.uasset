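; BP_Shop is a shop actor that stocks itself with randomly chosen items.
; UpdateShop loops over the direct child components of Arrow8 as spawn points and spawns a random ShopList class at each location, so repeats are possible.
; The chosen list index sets each item's ShopItemType, splitting the first three entries from the rest.
; Its event graph is empty and earlier spawns are not cleared.
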(event EventBeginPlay)

(event Collision|EventActorBeginOverlap
  (params (OtherActor :type Actor%20Object%20Reference)))

(event EventTick
  (params (DeltaSeconds :type Float%20%28single-precision%29)))

(fn ConstructionScript)

(fn UpdateShop
  (bind _shoplist (Variables|Default|GetShopList))
  (for _array_element (Components|GetChildrenComponents (Variables|Default|GetArrow8) false)
    (LocalVariables|SetNewLocalVar (Math|Random|RandomIntegerinRange 0 (- (Utilities|Array|Length _shoplist) 1)))
    (Game|SpawnActorfromClass (Utilities|Array|Get(acopy) _shoplist (LocalVariables|GetNewLocalVar)) (Math|Transform|MakeTransform (Transformation|GetWorldLocation _array_element)) "Undefined" "MultiplyWithRoot" 0 (select (> (LocalVariables|GetNewLocalVar) 2) "NewEnumerator0" "NewEnumerator1") 0)))