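; Wave actor Blueprint that animates a static mesh as a flipbook by swapping its material.
; On BeginPlay it loops endlessly through the first four entries of the NewVar material array, applying each to slot 0 of the mesh.
; Fixed short delays pace the frames, and the last delay wires back to the first material instead of using Tick or a timer.
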(event EventBeginPlay
  (Rendering|Material|SetMaterial (Variables|Debug|GetStaticMeshComponent) 0 (Utilities|Array|Get(acopy) (Variables|Default|GetNewVar)) :!label _label)
  (Utilities|FlowControl|Delay 0.2)
  (Rendering|Material|SetMaterial (Variables|Debug|GetStaticMeshComponent) 0 (Utilities|Array|Get(acopy) (Variables|Default|GetNewVar) 1))
  (Utilities|FlowControl|Delay 0.2)
  (Rendering|Material|SetMaterial (Variables|Debug|GetStaticMeshComponent) 0 (Utilities|Array|Get(acopy) (Variables|Default|GetNewVar) 2))
  (Utilities|FlowControl|Delay 0.2)
  (Rendering|Material|SetMaterial (Variables|Debug|GetStaticMeshComponent) 0 (Utilities|Array|Get(acopy) (Variables|Default|GetNewVar) 3))
  (Utilities|FlowControl|Delay 0.2)
  (goto _label))

(fn ConstructionScript)