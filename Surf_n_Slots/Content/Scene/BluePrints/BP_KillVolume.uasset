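; BP_KillVolume is a trigger volume that recycles overlapping actors by respawning them at the spawn volume's Y position.
; On BeginPlay it caches the first BP_SpawnVolume found in the level.
; On overlap it has that volume spawn a new instance of the actor's class, keeping X, Z, rotation and scale but taking the volume's Y.
; It then destroys the original, so no instance state is copied.
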(event OnComponentBeginOverlap(KillVolume)
  (params (OverlappedComponent :type Primitive%20Component%20Object%20Reference) (OtherActor :type Actor%20Object%20Reference) (OtherComp :type Primitive%20Component%20Object%20Reference) (OtherBodyIndex :type Integer) (bFromSweep :type Boolean) (SweepResult :type Hit%20Result%20Structure%20%28by%20ref%29))
  (bind _returnvalue (Transformation|GetActorTransform OtherActor))
  (bind _returnvalue_2 (Transformation|GetActorLocation OtherActor))
  (bind (_location _rotation _scale) (Math|Transform|BreakTransform _returnvalue))
  (bind (_x _y _z) (Math|Vector|BreakVector _returnvalue_2))
  (Utilities|IsValid OtherActor
    (:Is%20Valid
      (Default|SpawnObject (Variables|Default|GetSpawnVolume_ref) (Utilities|GetClass OtherActor) (Math|Transform|MakeTransform (Math|Vector|MakeVector _x (.Y (Math|Vector|BreakVector (Transformation|GetActorLocation (Variables|Default|GetSpawnVolume_ref)))) _z) _rotation _scale))
      (Actor|DestroyActor OtherActor))))

(event EventBeginPlay
  (bind _returnvalue (Actor|GetActorOfClass "/Game/Scene/BluePrints/BP_SpawnVolume.BP_SpawnVolume_C"))
  (Variables|Default|SetSpawnVolume_ref _returnvalue))

(event Collision|EventActorBeginOverlap
  (params (OtherActor :type Actor%20Object%20Reference)))

(event EventTick
  (params (DeltaSeconds :type Float%20%28single-precision%29)))

(fn ConstructionScript)